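; BP_AIBaseBot is a base AI bot that detects the player and reports it to the Blackboard.
; A looping timer started on BeginPlay runs a debug-drawn Camera-channel line trace toward the first player's pawn every 0.1 seconds.
; An unobstructed hit within close range sets the PlayerCharacter key to that pawn; otherwise the key is cleared.
; The AIPerception update event is empty, with its Blackboard write left disconnected.
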(event OnTargetPerceptionUpdated(AIPerception)
  (params (Actor :type Actor%20Object%20Reference) (Stimulus :type AI%20Stimulus%20Structure)))

(event Custom|TraceForPlayer
  (bind _outhit (Collision|LineTraceByChannel (Transformation|GetActorLocation) (Transformation|GetActorLocation (Pawn|GetControlledPawn (Game|GetPlayerController 0))) "TraceTypeQuery2" true 0 "ForDuration" true "(R=1.000000,G=0.000000,B=0.000000,A=1.000000)" "(R=0.000000,G=1.000000,B=0.000000,A=1.000000)" 2.0))
  (if (== (.HitActor (Collision|BreakHitResult _outhit)) (Pawn|GetControlledPawn (Game|GetPlayerController 0)))
    (if (< (.Distance (Collision|BreakHitResult _outhit)) 5e+02)
      (AI|Components|Blackboard|SetValueasObject (AI|GetBlackboard 0) (Utilities|Name|MakeLiteralName "PlayerCharacter") (Pawn|GetControlledPawn (Game|GetPlayerController 0)))
      (else
        (AI|Components|Blackboard|SetValueasObject (AI|GetBlackboard 0) (Utilities|Name|MakeLiteralName "PlayerCharacter") 0 :!label _label)))
    (else
      (goto _label))))

(event EventBeginPlay
  (Utilities|Time|SetTimerbyEvent (delegate Custom|TraceForPlayer) 0.1 true))

(fn ConstructionScript)