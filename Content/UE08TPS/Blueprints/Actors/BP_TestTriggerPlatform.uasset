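; Test trigger platform actor that turns its cube emissive green while activated and red otherwise.
; Box begin and end overlaps call a multicast event, which fires the trigger-activated dispatcher that the actor binds to its own material-switching handler at BeginPlay.
; An IsActivated RepNotify routes through the same multicast, though no graph here sets that variable, and the local-role checks are disconnected.
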(event OnComponentBeginOverlap(Box)
  (params (OverlappedComponent :type Primitive%20Component%20Object%20Reference) (OtherActor :type Actor%20Object%20Reference) (OtherComp :type Primitive%20Component%20Object%20Reference) (OtherBodyIndex :type Integer) (bFromSweep :type Boolean) (SweepResult :type Hit%20Result%20Structure%20%28by%20ref%29))
  (CallFunction|MulticastChangeColoronPlatform true))

(event OnComponentEndOverlap(Box)
  (params (OverlappedComponent :type Primitive%20Component%20Object%20Reference) (OtherActor :type Actor%20Object%20Reference) (OtherComp :type Primitive%20Component%20Object%20Reference) (OtherBodyIndex :type Integer))
  (CallFunction|MulticastChangeColoronPlatform false))

(event Custom|Multicast_ChangeColorOnPlatform
  (params (Active :type Boolean))
  (Default|CallTriggerActivatedd Active))

(event Custom|TriggerBox
  (params (isActivated :type Boolean))
  (bind _cube (Variables|Default|GetCube))
  (if isActivated
    (Rendering|Material|SetMaterial _cube 0 "/Game/UE08TPS/Materials/MI_Emissive_Green.MI_Emissive_Green")
    (else
      (Rendering|Material|SetMaterial _cube 0 "/Game/UE08TPS/Materials/MI_Emissive_Red.MI_Emissive_Red"))))

(event EventBeginPlay
  (EventDispatchers|BindEventtoTriggerActivatedd (delegate Custom|TriggerBox)))

(fn ConstructionScript)

(fn OnRepIsActivated
  (CallFunction|MulticastChangeColoronPlatform (Variables|Default|GetIsActivated)))