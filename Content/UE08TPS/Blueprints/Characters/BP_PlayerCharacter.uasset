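; BP_PlayerCharacter is the player character for UE08TPS, adding a crosshair HUD, world interaction and an inventory screen.
; BeginPlay creates the crosshair widget, and the interact input uses a short-range GetAimPoint hit to message actors implementing BPI_Interactable.
; The inventory input creates W_Inventory, fills its grid from the BACInventorySystem component, and clears the stored reference through the widget's OnClose event.
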(event Custom|ClearInventoryRef
  (Variables|Default|SetInventory_Ref 0))

(event Input|EnhancedActionEvents|EnhancedInputActionIA_UE08Interact
  (params (ActionValue :type Boolean) (ElapsedSeconds :type Float%20%28double-precision%29) (TriggeredSeconds :type Float%20%28double-precision%29) (InputAction :type Input%20Action%20Object%20Reference :default "/Game/UE08TPS/Input/Actions/IA_UE08Interact.IA_UE08Interact"))
  (bind _hitresult (Class|UE08BaseCharacter|GetAimPoint 5e+02))
  (bind (_bblockinghit _binitialoverlap _time _distance _location _impactpoint _normal _impactnormal _physmat _hitactor) (Collision|BreakHitResult _hitresult))
  (:Started
    (if _bblockinghit
      (if (Utilities|DoesObjectImplementInterface _hitactor "/Game/UE08TPS/Interfaces/BPI_Interactable.BPI_Interactable_C")
        (Class|BPIInteractable|Interact(Message) _hitactor self)))))

(event Input|EnhancedActionEvents|EnhancedInputActionIA_UE08Inventory
  (params (ActionValue :type Boolean) (ElapsedSeconds :type Float%20%28double-precision%29) (TriggeredSeconds :type Float%20%28double-precision%29) (InputAction :type Input%20Action%20Object%20Reference :default "/Game/UE08TPS/Input/Actions/IA_UE08Inventory.IA_UE08Inventory"))
  (:Started
    (bind _returnvalue (UserInterface|CreateWidget "/Game/UE08TPS/Widgets/Inventory/W_Inventory.W_Inventory_C"))
    (Variables|Default|SetInventory_Ref _returnvalue)
    (UserInterface|Viewport|AddtoViewport (Variables|Default|GetInventory_Ref) 0)
    (Default|DisplayInventory (Variables|/Game/UE08TPS/Widgets/Inventory/W_Inventory.W_Inventory_C|GetWBP_InventoryGrid (Variables|Default|GetInventory_Ref)) (Variables|Default|GetBAC_InventorySystem))
    (EventDispatchers|BindEventtoOnClose (Variables|Default|GetInventory_Ref) (delegate Custom|ClearInventoryRef))))

(event EventBeginPlay
  (bind _returnvalue (UserInterface|CreateWidget "/Game/UE08TPS/Blueprints/Characters/W_Crosshair.W_Crosshair_C" (Game|GetPlayerController 0)))
  (UserInterface|Viewport|AddtoViewport _returnvalue 0))

(fn ConstructionScript)