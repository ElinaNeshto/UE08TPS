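; BP_UE08Weapon is a third-person shooter weapon Blueprint that tints its point light by damage type in the construction script.
; Every tick it runs a line trace, but the hit-actor notify and trace response nodes are disconnected.
; BeginPlay binds a debug-print event to a custom delegate and fires it on a looping timer.
; A helper computes the maximum grab location along the actor's forward vector.
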(event Custom|ChangeColor
  (Development|PrintString "Hello, I'm delegate"))

(event Custom|CallDelegate
  (Default|CallMyBPDelegate))

(event EventBeginPlay
  (EventDispatchers|BindEventtoMyBPDelegate (delegate Custom|ChangeColor))
  (Utilities|Time|SetTimerbyEvent (delegate Custom|CallDelegate) 1e+01 true))

(event EventTick
  (params (DeltaSeconds :type Float%20%28single-precision%29))
  (bind (_hitresult _returnvalue) (Class|UE08Weapon|ThrowLineTrace))
  (if _returnvalue
    _))

(fn ConstructionScript
  (bind _pointlight (Variables|Default|GetPointLight))
  (switch Utilities|FlowControl|Switch|SwitchonEDamageType (Variables|Default|GetDamageType)
    (:Physical
      (Rendering|Components|Light|SetLightColor _pointlight "(R=0.152560,G=0.036458,B=1.000000,A=1.000000)" true))
    (:Fire
      (Rendering|Components|Light|SetLightColor _pointlight "(R=1.000000,G=0.274684,B=0.041667,A=1.000000)" true))
    (:Ice
      (Rendering|Components|Light|SetLightColor _pointlight "(R=0.026042,G=1.000000,B=0.888473,A=1.000000)" true))
    (:Explosion
      (Rendering|Components|Light|SetLightColor _pointlight "(R=0.682292,G=0.000000,B=0.016199,A=1.000000)" true))))

(fn GetMaxGrabLocation0
  (return (+ (Transformation|GetActorLocation) (* (Math|Vector|GetForwardVector (Transformation|GetActorRotation)) (Variables|Default|GetMaxGrabDistance)))))

(fn NotifyActor
  (params (Actor :type Actor%20Object%20Reference))
  (Development|PrintString (Utilities|GetDisplayName Actor)))