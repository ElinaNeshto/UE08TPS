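; BP_Item is a pickup item actor that moves into an interacting actor's inventory.
; On spawn its sphere simulates physics, and a looping timer switches simulation off once the body falls asleep.
; Interact passes its item ID and quantity to the actor's BAC_InventorySystem, destroying itself on success or keeping the remainder and printing a message.
; UseItem is an empty event.
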(event Custom|GetPhysicsAsleep
  (if (not (Class|PrimitiveComponent|IsAnyRigidBodyAwake (Variables|Default|GetSphere)))
    (Physics|SetSimulatePhysics (Variables|Default|GetSphere) false)
    (Utilities|Time|ClearandInvalidateTimerbyHandle (Variables|Default|GetPhysicsTimerHandle))))

(event Custom|UseItem
  (params (ActorToGetAbility :type Actor%20Object%20Reference)))

(event EventBeginPlay
  (Physics|SetSimulatePhysics (Variables|Default|GetSphere) true)
  (bind _returnvalue (Utilities|Time|SetTimerbyEvent (EventDispatchers|CreateEvent :!event Custom|GetPhysicsAsleep) 0.1 true))
  (Variables|Default|SetPhysicsTimerHandle _returnvalue))

(event EventInteract
  (params (Actor :type Actor%20Object%20Reference))
  (bind _returnvalue (Actor|GetComponentbyClass Actor "/Game/UE08TPS/Components/BAC_InventorySystem.BAC_InventorySystem_C"))
  (bind _bac_ieminventory (Variables|Default|GetBAC_IemInventory))
  (Utilities|IsValid _returnvalue
    (:Is%20Valid
      (bind (_issuccess _quantityremain) (Default|AddtoInventory _returnvalue (.rowname (Variables|/Game/UE08TPS/Components/BAC_IemInventory.BAC_IemInventory_C|GetItemData _bac_ieminventory)) (Variables|/Game/UE08TPS/Components/BAC_IemInventory.BAC_IemInventory_C|GetQuantity _bac_ieminventory)))
      (if _issuccess
        (Actor|DestroyActor)
        (else
          (Variables|/Game/UE08TPS/Components/BAC_IemInventory.BAC_IemInventory_C|SetQuantity (Variables|Default|GetBAC_IemInventory) _quantityremain)
          (if (== _quantityremain (Variables|/Game/UE08TPS/Components/BAC_IemInventory.BAC_IemInventory_C|GetQuantity _bac_ieminventory))
            (Development|PrintString "NO SPACE IN INVENTORY")
            (else
              (Development|PrintString "ONLY A FEW THINGS WAS TAKEN"))))))))

(fn ConstructionScript)