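; BP_UE08Effect is an effect Blueprint that assigns the AttributeReaderTrails Niagara system to its component at BeginPlay.
; It fetches the component through Component, then passes it to ComponentName to log the object name without screen output.
; ChangeParametrs swaps the asset and resets existing override parameters, falling back to the parent implementation when the component is invalid.
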(event EventBeginPlay
  (bind _niagara (Class|UE08Effect|Component))
  (Class|UE08Effect|ComponentName _niagara)
  (Class|UE08Effect|ChangeParametrs _niagara))

(event EventComponentName
  (params (Niagara :type Niagara%20Component%20Object%20Reference))
  (Utilities|IsValid Niagara
    (:Is%20Valid
      (Development|PrintString (Utilities|GetObjectName Niagara) false))))

(event EventChangeParametrs
  (params (Niagara :type Niagara%20Component%20Object%20Reference))
  (Utilities|IsValid Niagara
    (:Is%20Valid
      (Class|NiagaraComponent|SetAsset Niagara "/Niagara/DefaultAssets/Templates/Systems/AttributeReaderTrails.AttributeReaderTrails" true))
    (:Is%20Not%20Valid
      (|CallParentFunction 0))))

(fn ConstructionScript)